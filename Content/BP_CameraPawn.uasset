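; BP_CameraPawn is a camera pawn that the player can take over and cycle away from to the next or previous camera.
; InitializeMe spawns a default AI controller if none exists, caches it, and hands the pawn to it.
; TakeControll gives possession to player controller 0, and RemoveControll returns it to the cached AI controller.
; Next and previous camera Enhanced Input actions call SwitchCamera with a direction boolean, leaving the switching to other logic.
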(event `RemoveControll`
  (`Controller.Possess` (`self.Original_AI`) self))

(event `TakeControll`
  (`Controller.Possess` (`GameplayStatics.GetPlayerController` 0) self))

(event `EnhancedInput|/Game/Input/IA_PreviousCamera`
  (params (ActionValue :type Boolean) (ElapsedSeconds :type "Float (double-precision)") (TriggeredSeconds :type "Float (double-precision)") (InputAction :type "InputAction Object Reference" :default "/Game/Input/IA_PreviousCamera.IA_PreviousCamera"))
  (:`Triggered`
    (`self.SwitchCamera` false)))

(event `EnhancedInput|/Game/Input/IA_NextCamera`
  (params (ActionValue :type Boolean) (ElapsedSeconds :type "Float (double-precision)") (TriggeredSeconds :type "Float (double-precision)") (InputAction :type "InputAction Object Reference" :default "/Game/Input/IA_NextCamera.IA_NextCamera"))
  (:`Triggered`
    (`self.SwitchCamera` true)))

(fn `InitializeMe`
  (bind _returnvalue (`AIBlueprintHelperLibrary.GetAIController` self))
  (if (not (`KismetSystemLibrary.IsValid` _returnvalue))
    (`self.SpawnDefaultController`))
  (set `self.Original_AI` _returnvalue)
  (`self.RemoveControll`))

(fn `UserConstructionScript`)